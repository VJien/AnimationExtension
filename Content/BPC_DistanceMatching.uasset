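; BPC_DistanceMatching is a component that tracks a character's acceleration state to supply reference data for distance matching of jog starts and stops.
; UpdateDistanceMatching detects changes in horizontal acceleration through the movement component cached by Init.
; On start it saves the current location; on stop it predicts the stop location from braking physics, resetting the matching curve time each way.
; EvalDistanceMatching and UpdateCurveValue are empty stubs.
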(event EventBeginPlay)

(event EventTick
  (params (DeltaSeconds :type Float%20%28single-precision%29)))

(fn Init
  (params (Character :type Character%20Object%20Reference))
  (bind _output_get (Variables|Default|SetCharacter Character))
  (Variables|Default|SetCharacter%20Movement%20Component (Variables|/Script/Engine.Character|GetCharacterMovement _output_get)))

(fn UpdateDistanceMatching
  (bind _character_movement_component (Variables|Default|GetCharacter%20Movement%20Component))
  (Variables|Default|GetCharacter%20Movement%20Component
    (:then
      (Variables|Default|SetbCurrentIsAccelerating (> (Class|KismetMathLibrary|VSizeXYSquared (Pawn|Components|CharacterMovement|GetCurrentAcceleration (Variables|Default|GetCharacter%20Movement%20Component))) 0.0))
      (if (not (Math|Boolean|Equal(Boolean) (Variables|Default|GetbCurrentIsAccelerating) (Variables|Default|GetbIsAccelerating)))
        (bind _output_get (Variables|Default|SetbIsAccelerating (Variables|Default|GetbCurrentIsAccelerating)))
        (if _output_get
          (Variables|Default|SetJogDistanceCurveStartTime 0.0)
          (Variables|Default|SetDistanceMachingLocation (Transformation|GetActorLocation (Variables|Default|GetCharacter)))
          (else
            (Variables|Default|SetJogDistanceCurveStopTime 0.0)
            (bind _outstoplocation (Class|AnimExtensionBlueprintLibrary|PredictStopLocation (Transformation|GetActorLocation (Variables|Default|GetCharacter)) (Variables|/Script/Engine.MovementComponent|GetVelocity _character_movement_component) (Pawn|Components|CharacterMovement|GetCurrentAcceleration _character_movement_component) (Variables|/Script/Engine.CharacterMovementComponent|GetBrakingFriction _character_movement_component) (Class|CharacterMovementComponent|GetMaxBrakingDeceleration _character_movement_component) (Variables|/Script/Engine.CharacterMovementComponent|GetMaxSimulationTimeStep _character_movement_component) (Variables|Default|GetMax%20Simulation%20Iterations)))
            (Variables|Default|SetDistanceMachingLocation _outstoplocation)))))
    (:else)))

(fn EvalDistanceMatching
  (params (deltaX :type Float%20%28single-precision%29)))

(fn UpdateCurveValue
  (params (InputX :type Float%20%28single-precision%29) (InputY :type Float%20%28single-precision%29) (bOrient%20Rotation%20to%20Movement :type Boolean)))